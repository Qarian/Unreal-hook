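; LocationMarker is a level volume that registers a named location with the FirstPersonCharacter while it is inside.
; Begin overlap calls AddLocation with the marker's Name on the character, and end overlap calls RemoveLocation with the same Name.
; The construction script creates a dynamic material on the Cube and tints it with EditorColor, giving each marker its own color.
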(event Collision|EventActorBeginOverlap
  (params (OtherActor :type Actor%20Object%20Reference))
  (bind _asfirst_person_character (Utilities|Casting|CastToFirstPersonCharacter OtherActor))
  (Default|AddLocation _asfirst_person_character (Variables|Location|GetName)))

(event Collision|EventActorEndOverlap
  (params (OtherActor :type Actor%20Object%20Reference))
  (bind _asfirst_person_character (Utilities|Casting|CastToFirstPersonCharacter OtherActor))
  (Default|RemoveLocation _asfirst_person_character (Variables|Location|GetName)))

(fn ConstructionScript
  (bind _returnvalue (Rendering|Material|CreateDynamicMaterialInstance (Variables|Default|GetCube) 0 0 "None" :!class /Script/Engine.PrimitiveComponent))
  (Rendering|Material|SetVectorParameterValue _returnvalue "Color" (Variables|Location|GetEditor%20color) :!class /Script/Engine.MaterialInstanceDynamic))