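; Pressure plate actor that moves a linked MovedObject by DistanceToMove while actors stand on it.
; Overlaps increment a counter, tint the plate active through a dynamic material instance and play a timeline that lerps the object from its starting location.
; When the counter returns to zero, the plate reverts to its inactive color and the timeline reverses.
; The end position is recomputed on each overlap, so the distance can change during gameplay.
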(event EventBeginPlay
  (Utilities|SetPlateColor (Variables|Colors|GetInactive%20Color))
  (Variables|Default|SetStart%20position (Transformation|GetActorLocation (Variables|Elevator|GetMoved%20Object))))

(event Collision|EventActorBeginOverlap
  (params (OtherActor :type Actor%20Object%20Reference))
  (Math|Integer|IncrementInt (Variables|Default|GetActors%20Above%20Count)
    (:%20%20
      (Utilities|SetPlateColor (Variables|Colors|GetActive%20Color))
      ;[1 1 1] Calculate here to enable changing value mid gameplay
      (Variables|Default|SetEnd%20position (+ (Variables|Default|GetStart%20position) (Variables|Elevator|GetDistance%20to%20move)))
      (bind _progress (Timeline|Triggered%20movement Play)
        (:Update
          (Transformation|SetActorLocation (Variables|Elevator|GetMoved%20Object) (Math|Vector|Lerp(Vector) (Variables|Default|GetStart%20position) (Variables|Default|GetEnd%20position) _progress) false false))))))

(event Collision|EventActorEndOverlap
  (params (OtherActor :type Actor%20Object%20Reference))
  (bind _result (Math|Integer|DecrementInt (Variables|Default|GetActors%20Above%20Count))
    (:%20%20
      (if (== _result 0)
        (Utilities|SetPlateColor (Variables|Colors|GetInactive%20Color))
        (bind _progress (Timeline|Triggered%20movement Reverse)
          (:Update
            (Transformation|SetActorLocation (Variables|Elevator|GetMoved%20Object) (Math|Vector|Lerp(Vector) (Variables|Default|GetStart%20position) (Variables|Default|GetEnd%20position) _progress) false false)))))))

(fn ConstructionScript)